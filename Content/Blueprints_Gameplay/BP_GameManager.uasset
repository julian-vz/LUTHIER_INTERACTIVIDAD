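; Game manager that runs a step-by-step guitar-building sequence, apparently in VR, from intro narration to return to menu.
; Each BPTriggerBoxRef completion advances CurrentTask, dims a spotlight and plays dialogue, whose finish callback lights and enables the next station.
; Most steps spawn guitar parts at MesaRef, with top and rim materials set by wood selection.
; The last task spawns the finished guitar, then plays a Level Sequence before loading VRTemplateMenu.
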(event `self.ReceiveBeginPlay`
  (`|ExecutionSequence`
    (:`then_0`
      ; Paso 1 Tapa
      (`KismetSystemLibrary.Delay` 8.0)
      ;; Audio
      (bind _output_get (set `self.DialogueType` "NewEnumerator0"))
      (bind _returnvalue (`GameplayStatics.GetActorOfClass` "/Game/Audios/BP_AudioManagerMain.BP_AudioManagerMain_C"))
      (bind _dialoguefinished (`/Game/Audios/BP_AudioManagerMain.PlayDialogue` _returnvalue _output_get))
      (add `AudioComponent.OnAudioFinished` _dialoguefinished (delegate `AudioFinished`)))
    (:`then_1`
      (for _array_element (`self.BP_TriggerBox_Ref`)
        (add `/Game/Blueprints_Escenario/BP_TriggerBox.TaskCompleted` _array_element (delegate `onTaskCompleted`))))
    (:`then_2`
      (`GameplayStatics.SetSoundMixClassOverride` "/Game/Audios/SM_Global.SM_Global" "/Game/Audios/SC_Master.SC_Master" 3.0)
      (`GameplayStatics.PushSoundMixModifier` "/Game/Audios/SM_Global.SM_Global"))))

(event `AudioFinished`
  ; Paso 1 Tapa
  ;; Audio
  (`KismetSystemLibrary.Delay` 1.0)
  ;; Luz on
  (`GameplayStatics.GetAllActorsOfClass` "/Game/Blueprints_Escenario/Spotlight.Spotlight_C")
  (`LightComponent.SetIntensity` (`/Game/Blueprints_Escenario/Spotlight.SpotLight` (`|GetArrayItem` (`self.Light`) 1)) 60000.0)
  (set `/Game/Blueprints_Escenario/BP_TriggerBox.bTriggerEnabled` true (`|GetArrayItem` (`self.BP_TriggerBox_Ref`))))

(event `onTaskCompleted`
  (bind _guitarra_spawn (`self.Guitarra_Spawn`))
  (bind _guitarraspawned_ref (`self.GuitarraSpawned_Ref`))
  (bind _returnvalue (`self.GetTransform` (`self.Mesa_Ref`)))
  (bind _result (`/Engine/EditorBlueprintResources/StandardMacros.IncrementInt` (`self.CurrentTask`))
    (:`  `
      (switch `int` _result
        (:`1`
          ; Paso 2 Lijado
          (bind _returnvalue_2 (`|SpawnActorFromClass` "/Game/Blueprints_Escenario/BP_GuitarraCentral.BP_GuitarraCentral_C" (`self.GetTransform` (`self.Mesa_Ref`)) "Undefined" "MultiplyWithRoot" null (`|GetArrayItem` (`self.Guitarra_Spawn`)) null))
          (switch `/Game/Blueprints_Gameplay/EN_MaderaTapa` (`self.Selec_Tapa`)
            (:`NewEnumerator0`
              (bind _staticmesh (`/Game/Blueprints_Escenario/BP_GuitarraCentral.StaticMesh` _returnvalue_2))
              (`PrimitiveComponent.SetMaterial` _staticmesh 0 "/Game/Materiales/Material_003.Material_003"))
            (:`NewEnumerator1`
              (`PrimitiveComponent.SetMaterial` _staticmesh 0 "/Game/Materiales/MI_Material_003Instance.MI_Material_003Instance")))
          (`KismetArrayLibrary.Array_Add` (`self.GuitarraSpawned_Ref`))
          (`KismetSystemLibrary.Delay` 2.0)
          (`|ExecutionSequence`
            (:`then_0`
              ; Paso 1 Tapa
              ;; Luz off
              (`GameplayStatics.GetAllActorsOfClass` "/Game/Blueprints_Escenario/Spotlight.Spotlight_C")
              (`LightComponent.SetIntensity` (`/Game/Blueprints_Escenario/Spotlight.SpotLight` (`|GetArrayItem` (`self.Light`) 1)) 0.0))
            (:`then_1`
              ;; Audio
              (bind _output_get (set `self.DialogueType` "NewEnumerator1"))
              (bind _returnvalue_3 (`GameplayStatics.GetActorOfClass` "/Game/Audios/BP_AudioManagerMain.BP_AudioManagerMain_C"))
              (bind _dialoguefinished (`/Game/Audios/BP_AudioManagerMain.PlayDialogue` _returnvalue_3 _output_get))
              (add `AudioComponent.OnAudioFinished` _dialoguefinished (delegate `CustomEvent2`)))))
        (:`2`
          ; Paso 3 Varetaje
          (`KismetSystemLibrary.Delay` 2.0)
          (`|ExecutionSequence`
            (:`then_0`
              ;; Luz off
              (`GameplayStatics.GetAllActorsOfClass` "/Game/Blueprints_Escenario/Spotlight.Spotlight_C")
              (`LightComponent.SetIntensity` (`/Game/Blueprints_Escenario/Spotlight.SpotLight` (`|GetArrayItem` (`self.Light`) 2)) 0.0))
            (:`then_1`
              ;; Audio
              (bind _output_get_2 (set `self.DialogueType` "NewEnumerator2"))
              (bind _returnvalue_4 (`GameplayStatics.GetActorOfClass` "/Game/Audios/BP_AudioManagerMain.BP_AudioManagerMain_C"))
              (bind _dialoguefinished_2 (`/Game/Audios/BP_AudioManagerMain.PlayDialogue` _returnvalue_4 _output_get_2))
              (add `AudioComponent.OnAudioFinished` _dialoguefinished_2 (delegate `CustomEvent 3`)))))
        (:`3`
          ; Paso 4 Mastil
          (bind _returnvalue_5 (`|SpawnActorFromClass` "/Game/Blueprints_Escenario/BP_GuitarraCentral.BP_GuitarraCentral_C" (`self.GetTransform` (`self.Mesa_Ref`)) "Undefined" "MultiplyWithRoot" null (`|GetArrayItem` (`self.Guitarra_Spawn`) 1) null))
          (`KismetArrayLibrary.Array_Add` (`self.GuitarraSpawned_Ref`) _returnvalue_5)
          (`KismetSystemLibrary.Delay` 2.0)
          (`|ExecutionSequence`
            (:`then_0`
              ;; Luz off
              (`GameplayStatics.GetAllActorsOfClass` "/Game/Blueprints_Escenario/Spotlight.Spotlight_C")
              (`LightComponent.SetIntensity` (`/Game/Blueprints_Escenario/Spotlight.SpotLight` (`|GetArrayItem` (`self.Light`) 3)) 0.0))
            (:`then_1`
              ;; Audio
              (bind _output_get_3 (set `self.DialogueType` "NewEnumerator3"))
              (bind _returnvalue_6 (`GameplayStatics.GetActorOfClass` "/Game/Audios/BP_AudioManagerMain.BP_AudioManagerMain_C"))
              (bind _dialoguefinished_3 (`/Game/Audios/BP_AudioManagerMain.PlayDialogue` _returnvalue_6 _output_get_3))
              (add `AudioComponent.OnAudioFinished` _dialoguefinished_3 (delegate `CustomEvent 4`)))))
        (:`4`
          ; Paso 5 Aros
          (bind _returnvalue_7 (`|SpawnActorFromClass` "/Game/Blueprints_Escenario/BP_GuitarraCentral.BP_GuitarraCentral_C" (`self.GetTransform` (`self.Mesa_Ref`)) "Undefined" "MultiplyWithRoot" null (`|GetArrayItem` (`self.Guitarra_Spawn`) 2) null))
          (`KismetArrayLibrary.Array_Add` (`self.GuitarraSpawned_Ref`) _returnvalue_7)
          (`KismetSystemLibrary.Delay` 2.0)
          (`|ExecutionSequence`
            (:`then_0`
              ;; Luz off
              (`GameplayStatics.GetAllActorsOfClass` "/Game/Blueprints_Escenario/Spotlight.Spotlight_C")
              (`LightComponent.SetIntensity` (`/Game/Blueprints_Escenario/Spotlight.SpotLight` (`|GetArrayItem` (`self.Light`) 3)) 0.0))
            (:`then_1`
              ;; Audio
              (bind _output_get_4 (set `self.DialogueType` "NewEnumerator4"))
              (bind _returnvalue_8 (`GameplayStatics.GetActorOfClass` "/Game/Audios/BP_AudioManagerMain.BP_AudioManagerMain_C"))
              (bind _dialoguefinished_4 (`/Game/Audios/BP_AudioManagerMain.PlayDialogue` _returnvalue_8 _output_get_4))
              (add `AudioComponent.OnAudioFinished` _dialoguefinished_4 (delegate `CustomEvent 5`)))))
        (:`5`
          ; Paso 6 Trastes
          (bind _returnvalue_9 (`|SpawnActorFromClass` "/Game/Blueprints_Escenario/BP_GuitarraCentral.BP_GuitarraCentral_C" _returnvalue "Undefined" "MultiplyWithRoot" null (`|GetArrayItem` _guitarra_spawn 3) null))
          (`KismetArrayLibrary.Array_Add` _guitarraspawned_ref _returnvalue_9)
          (bind _returnvalue_10 (`|SpawnActorFromClass` "/Game/Blueprints_Escenario/BP_GuitarraCentral.BP_GuitarraCentral_C" _returnvalue "Undefined" "MultiplyWithRoot" null (`|GetArrayItem` _guitarra_spawn 4) null))
          (`KismetArrayLibrary.Array_Add` _guitarraspawned_ref _returnvalue_10)
          (switch `/Game/Blueprints_Gameplay/EN_MaderaAros` (`self.Selec_Aros`)
            (:`NewEnumerator0`
              (bind _staticmesh_2 (`/Game/Blueprints_Escenario/BP_GuitarraCentral.StaticMesh` _returnvalue_9))
              (`PrimitiveComponent.SetMaterial` _staticmesh_2 0 "/Game/Materiales/Material_003.Material_003"))
            (:`NewEnumerator1`
              (`PrimitiveComponent.SetMaterial` _staticmesh_2 0 "/Game/Materiales/MI_Material_003Instance.MI_Material_003Instance")))
          (`KismetSystemLibrary.Delay` 2.0)
          (`|ExecutionSequence`
            (:`then_0`
              ;; Luz off
              (`GameplayStatics.GetAllActorsOfClass` "/Game/Blueprints_Escenario/Spotlight.Spotlight_C")
              (`LightComponent.SetIntensity` (`/Game/Blueprints_Escenario/Spotlight.SpotLight` (`|GetArrayItem` (`self.Light`) 4)) 0.0))
            (:`then_1`
              ;; Audio
              (bind _output_get_5 (set `self.DialogueType` "NewEnumerator5"))
              (bind _returnvalue_11 (`GameplayStatics.GetActorOfClass` "/Game/Audios/BP_AudioManagerMain.BP_AudioManagerMain_C"))
              (bind _dialoguefinished_5 (`/Game/Audios/BP_AudioManagerMain.PlayDialogue` _returnvalue_11 _output_get_5))
              (add `AudioComponent.OnAudioFinished` _dialoguefinished_5 (delegate `CustomEvent 6`)))))
        (:`6`
          ; Paso 7
          (bind _returnvalue_12 (`|SpawnActorFromClass` "/Game/Blueprints_Escenario/BP_GuitarraCentral.BP_GuitarraCentral_C" (`self.GetTransform` (`self.Mesa_Ref`)) "Undefined" "MultiplyWithRoot" null (`|GetArrayItem` (`self.Guitarra_Spawn`) 5) null))
          (`KismetArrayLibrary.Array_Add` (`self.GuitarraSpawned_Ref`) _returnvalue_12)
          (`KismetSystemLibrary.Delay` 2.0)
          (`|ExecutionSequence`
            (:`then_0`
              ;; Luz off
              (`GameplayStatics.GetAllActorsOfClass` "/Game/Blueprints_Escenario/Spotlight.Spotlight_C")
              (`LightComponent.SetIntensity` (`/Game/Blueprints_Escenario/Spotlight.SpotLight` (`|GetArrayItem` (`self.Light`) 5)) 0.0))
            (:`then_1`
              ;; Audio
              (bind _output_get_6 (set `self.DialogueType` "NewEnumerator6"))
              (bind _returnvalue_13 (`GameplayStatics.GetActorOfClass` "/Game/Audios/BP_AudioManagerMain.BP_AudioManagerMain_C"))
              (bind _dialoguefinished_6 (`/Game/Audios/BP_AudioManagerMain.PlayDialogue` _returnvalue_13 _output_get_6))
              (add `AudioComponent.OnAudioFinished` _dialoguefinished_6 (delegate `CustomEvent 7`)))))
        (:`7`
          (`self.K2_DestroyActor` (`self.Guitarra_Elminación`))
          (`|SpawnActorFromClass` "/Game/Blueprints_Escenario/Guitarra_final.Guitarra_final_C" (`KismetMathLibrary.MakeTransform` (+ (`self.K2_GetActorLocation` (`self.Mesa_Ref`)) (0.0 -100.0 0.0)) (struct :`Yaw` -90.0)) "Undefined" "MultiplyWithRoot" null null)
          ; Fin
          (`KismetSystemLibrary.Delay` 0.2)
          (`|ExecutionSequence`
            (:`then_0`
              ;; Luz off
              (`GameplayStatics.GetAllActorsOfClass` "/Game/Blueprints_Escenario/Spotlight.Spotlight_C")
              (`LightComponent.SetIntensity` (`/Game/Blueprints_Escenario/Spotlight.SpotLight` (`|GetArrayItem` (`self.Light`) 6)) 0.0))
            (:`then_1`
              ;; Audio
              (bind _output_get_7 (set `self.DialogueType` "NewEnumerator7"))
              (bind _returnvalue_14 (`GameplayStatics.GetActorOfClass` "/Game/Audios/BP_AudioManagerMain.BP_AudioManagerMain_C"))
              (bind _dialoguefinished_7 (`/Game/Audios/BP_AudioManagerMain.PlayDialogue` _returnvalue_14 _output_get_7))
              (add `AudioComponent.OnAudioFinished` _dialoguefinished_7 (delegate `CustomEvent 8`)))))))))

(event `CustomEvent2`
  ; Paso 2 Lijado
  ;; Audio
  (`KismetSystemLibrary.Delay` 1.0)
  ;; Luz
  (`GameplayStatics.GetAllActorsOfClass` "/Game/Blueprints_Escenario/Spotlight.Spotlight_C")
  (`LightComponent.SetIntensity` (`/Game/Blueprints_Escenario/Spotlight.SpotLight` (`|GetArrayItem` (`self.Light`) 2)) 60000.0)
  (set `/Game/Blueprints_Escenario/BP_TriggerBox.bTriggerEnabled` true (`|GetArrayItem` (`self.BP_TriggerBox_Ref`) 1)))

(event `CustomEvent 3`
  ; Paso 3 Varetaje
  ;; Audio
  (`KismetSystemLibrary.Delay` 1.0)
  ;; Luz
  (`GameplayStatics.GetAllActorsOfClass` "/Game/Blueprints_Escenario/Spotlight.Spotlight_C")
  (`LightComponent.SetIntensity` (`/Game/Blueprints_Escenario/Spotlight.SpotLight` (`|GetArrayItem` (`self.Light`) 3)) 60000.0)
  (set `/Game/Blueprints_Escenario/BP_TriggerBox.bTriggerEnabled` true (`|GetArrayItem` (`self.BP_TriggerBox_Ref`) 2)))

(event `CustomEvent 4`
  ; Paso 4 Mastil
  ;; Audio
  (`KismetSystemLibrary.Delay` 1.0)
  ;; Luz
  (`GameplayStatics.GetAllActorsOfClass` "/Game/Blueprints_Escenario/Spotlight.Spotlight_C")
  (`LightComponent.SetIntensity` (`/Game/Blueprints_Escenario/Spotlight.SpotLight` (`|GetArrayItem` (`self.Light`) 3)) 60000.0)
  (set `/Game/Blueprints_Escenario/BP_TriggerBox.bTriggerEnabled` true (`|GetArrayItem` (`self.BP_TriggerBox_Ref`) 3)))

(event `CustomEvent 5`
  ; Paso 5 Aros
  ;; Audio
  (`KismetSystemLibrary.Delay` 1.0)
  ;; Luz
  (`GameplayStatics.GetAllActorsOfClass` "/Game/Blueprints_Escenario/Spotlight.Spotlight_C")
  (`LightComponent.SetIntensity` (`/Game/Blueprints_Escenario/Spotlight.SpotLight` (`|GetArrayItem` (`self.Light`) 4)) 60000.0)
  (set `/Game/Blueprints_Escenario/BP_TriggerBox.bTriggerEnabled` true (`|GetArrayItem` (`self.BP_TriggerBox_Ref`) 4)))

(event `CustomEvent 6`
  ; Paso 6 Trastes
  ;; Audio
  (`KismetSystemLibrary.Delay` 1.0)
  ;; Luz
  (`GameplayStatics.GetAllActorsOfClass` "/Game/Blueprints_Escenario/Spotlight.Spotlight_C")
  (`LightComponent.SetIntensity` (`/Game/Blueprints_Escenario/Spotlight.SpotLight` (`|GetArrayItem` (`self.Light`) 5)) 60000.0)
  (set `/Game/Blueprints_Escenario/BP_TriggerBox.bTriggerEnabled` true (`|GetArrayItem` (`self.BP_TriggerBox_Ref`) 5)))

(event `CustomEvent 7`
  ; Paso 7
  ;; Audio
  (`KismetSystemLibrary.Delay` 1.0)
  ;; Luz
  (`GameplayStatics.GetAllActorsOfClass` "/Game/Blueprints_Escenario/Spotlight.Spotlight_C")
  (`LightComponent.SetIntensity` (`/Game/Blueprints_Escenario/Spotlight.SpotLight` (`|GetArrayItem` (`self.Light`) 6)) 60000.0)
  (set `/Game/Blueprints_Escenario/BP_TriggerBox.bTriggerEnabled` true (`|GetArrayItem` (`self.BP_TriggerBox_Ref`) 6)))

(event `CustomEvent 8`
  ; Fin
  ;; Audio
  (`KismetSystemLibrary.Delay` 3.0)
  (`MovieSceneSequencePlayer.Play` (`LevelSequenceActor.SequencePlayer` (`self.LevelSequence`)))
  (`KismetSystemLibrary.Delay` 5.0)
  (`GameplayStatics.OpenLevel` "VRTemplateMenu"))

(fn `UserConstructionScript`)