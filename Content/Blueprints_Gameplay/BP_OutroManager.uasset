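; Outro manager that runs the timed VR credits sequence on BeginPlay, then returns to the VRMenu level.
; It hides the controller widget debug lines, opens the animated text media and plays credits audio at the table reference actor.
; After a long delay it unhides three credits actor classes, then loops through seven spotlights, lighting each with a foley sound from BP_AudioManagerOutro.
; A FadeToBlack sequence precedes the level change.
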(event `self.ReceiveBeginPlay`
  (bind _index (`self.Index`))
  (bind _output (`|GetArrayItem` (`self.Light`) _index))
  (`|ExecutionSequence`
    (:`then_0`
      ;[0.1666 0.01975 0.2391 0.5] Apagar Debug Lines del Control
      (bind _asvrpawn (cast `/Game/VRTemplate/Blueprints/VRPawn` (`Controller.K2_GetPawn` (`GameplayStatics.GetPlayerController` 0))))
      (set `WidgetInteractionComponent.bShowDebug` false (`/Game/VRTemplate/Blueprints/VRPawn.WidgetInteractionRight` _asvrpawn))
      (set `WidgetInteractionComponent.bShowDebug` false (`/Game/VRTemplate/Blueprints/VRPawn.WidgetInteractionLeft` _asvrpawn)))
    (:`then_1`
      (`KismetSystemLibrary.Delay` 1.0)
      (`MediaPlayer.OpenSource` (`self.Media`) "/Game/Widgets/VideoFrase/FMS_Animación_Textos.FMS_Animación_Textos")
      (bind _outactors (`GameplayStatics.GetAllActorsOfClass` "/Game/Blueprints_Escenario/BP_ReferenciaMesa.BP_ReferenciaMesa_C"))
      (`GameplayStatics.PlaySoundAtLocation` "/Game/Audios/Diálogos/MS_Créditos.MS_Créditos" (`self.K2_GetActorLocation` (`|GetArrayItem` _outactors)) (struct) 1.0 1.0 0.0 null null null null)
      (`KismetSystemLibrary.Delay` 20.5)
      (`|ExecutionSequence`
        (:`then_0`
          ;[0.04519 0.4969 0.3968 0.502] Spawn Créditos 1
          (bind _outactors_2 (`GameplayStatics.GetAllActorsOfClass` "/Game/Widgets/Outro/BP_CréditosOutro1.BP_CréditosOutro1_C"))
          (for _array_element _outactors_2
            (bind `_asbp_créditos_outro_1` (cast `/Game/Widgets/Outro/BP_CréditosOutro1` _array_element))
            (`self.SetActorHiddenInGame` `_asbp_créditos_outro_1` false)))
        (:`then_1`
          ;[0.04519 0.4969 0.3968 0.502] Spawn Créditos 1
          (bind _outactors_3 (`GameplayStatics.GetAllActorsOfClass` "/Game/Widgets/Outro/BP_CréditosOutro2.BP_CréditosOutro2_C"))
          (for _array_element_2 _outactors_3
            (bind `_asbp_créditos_outro_2` (cast `/Game/Widgets/Outro/BP_CréditosOutro2` _array_element_2))
            (`self.SetActorHiddenInGame` `_asbp_créditos_outro_2` false)))
        (:`then_2`
          ;[0.04519 0.4969 0.3968 0.502] Spawn Créditos 1
          (bind _outactors_4 (`GameplayStatics.GetAllActorsOfClass` "/Game/Widgets/Outro/BP_CréditosOutro3.BP_CréditosOutro3_C"))
          (for _array_element_3 _outactors_4
            (bind `_asbp_créditos_outro_3` (cast `/Game/Widgets/Outro/BP_CréditosOutro3` _array_element_3))
            (`self.SetActorHiddenInGame` `_asbp_créditos_outro_3` false)))
        (:`then_3`
          (`KismetSystemLibrary.Delay` 0.2)
          ;[0.6172 0.2918 0.08228 0.502] Encendido Luces
          (`GameplayStatics.GetAllActorsOfClass` "/Game/Blueprints_Escenario/Spotlight.Spotlight_C" :!label _label)
          (`LightComponent.SetIntensity` (`/Game/Blueprints_Escenario/Spotlight.SpotLight` _output) 5000.0)
          ;;[0.5271 0.07227 0.07036 0.502] Sonido Luz
          (bind _returnvalue (`GameplayStatics.GetActorOfClass` "/Game/Audios/BP_AudioManagerOutro.BP_AudioManagerOutro_C"))
          (`/Game/Audios/BP_AudioManagerOutro.PlayFoley` _returnvalue (`self.PropType`) (`self.K2_GetActorLocation` _output))
          (bind _output_get (set `self.Index` (+ _index 1)))
          (if (>= _output_get 7)
            (`KismetSystemLibrary.Delay` 6.0)
            ;[0 0 0 0.7294] FadeOut
            (`MovieSceneSequencePlayer.Play` (`LevelSequenceActor.SequencePlayer` (`self.FadeToBlack`)))
            (`KismetSystemLibrary.Delay` 3.0)
            (`GameplayStatics.OpenLevel` "VRMenu")
            (else
              (`KismetSystemLibrary.Delay` 3.0)
              (goto _label))))))))

(fn `UserConstructionScript`)