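; BP_TriggerBox is a trigger volume that completes a task when an actor overlaps its Box while TriggerEnabled is set.
; If ActorReference[0] is valid, any overlapping actor completes it; otherwise, matches with the second or third reference may set SelecTapa or SelecAros on BP_GameManager, depending on their current values.
; Completion plays a check sound, destroys the overlapping actor, disables collision after a short delay, calls TaskCompleted and destroys itself.
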(event `self.ReceiveActorBeginOverlap`
  (params (OtherActor :type "Actor Object Reference")))

(event `self.Box.OnComponentBeginOverlap`
  (params (OverlappedComponent :type "PrimitiveComponent Object Reference") (OtherActor :type "Actor Object Reference") (OtherComp :type "PrimitiveComponent Object Reference") (OtherBodyIndex :type Integer) (bFromSweep :type Boolean) (SweepResult :type "HitResult Structure (by ref)"))
  (bind _actorreference (`self.ActorReference`))
  (if (`self.bTriggerEnabled`)
    (bind _outactors (`GameplayStatics.GetAllActorsOfClass` "/Game/Blueprints_Gameplay/BP_GameManager.BP_GameManager_C"))
    (`/Engine/EditorBlueprintResources/StandardMacros.IsValid` (`|GetArrayItem` _actorreference)
      (:`Is Valid`
        (`GameplayStatics.PlaySound2D` "/Game/Audios/Otros/MS_SonidoCheck.MS_SonidoCheck" 1.0 1.0 0.0 null null :!label _label)
        (`self.K2_DestroyActor` OtherActor)
        (`KismetSystemLibrary.Delay` 0.1)
        (`PrimitiveComponent.SetCollisionEnabled` (`self.Box`) "NoCollision")
        (`self.TaskCompleted`)
        (`self.K2_DestroyActor`))
      (:`Is Not Valid`
        (if (== OtherActor (`|GetArrayItem` _actorreference 1))
          (bind _output (`|GetArrayItem` _outactors))
          (bind _returnvalue (== (`/Game/Blueprints_Gameplay/BP_GameManager.Selec_Tapa` _output) 0))
          (if _returnvalue
            (set `/Game/Blueprints_Gameplay/BP_GameManager.Selec_Tapa` "NewEnumerator0" _output)
            (goto _label)
            (else
              (bind _returnvalue_2 (== (`/Game/Blueprints_Gameplay/BP_GameManager.Selec_Aros` _output) 0))
              (if _returnvalue_2
                (set `/Game/Blueprints_Gameplay/BP_GameManager.Selec_Aros` "NewEnumerator1" _output)
                (goto _label))))
          (elif (== OtherActor (`|GetArrayItem` _actorreference 2))
            (if _returnvalue
              (set `/Game/Blueprints_Gameplay/BP_GameManager.Selec_Tapa` "NewEnumerator1" _output)
              (goto _label)
              (elif _returnvalue_2
                (set `/Game/Blueprints_Gameplay/BP_GameManager.Selec_Aros` "NewEnumerator0" _output)
                (goto _label)))))))))

(fn `UserConstructionScript`)