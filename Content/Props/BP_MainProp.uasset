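; BP_MainProp is a grabbable prop that guides the player through task steps with highlights and audio.
; Tick enables custom depth on the mesh while the GameManager's CurrentTaskGlow matches its PasoRequerido and it is not held.
; Grabbing plays foley; on the matching step it also reveals the TrigerDestino destination mesh and, after a short delay, plays one-time dialogue through the AudioManager.
; Dropping hides the destination mesh.
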(event `self.ReceiveBeginPlay`)

(event `self.ReceiveTick`
  (params (DeltaSeconds :type "Float (single-precision)"))
  (bind _itemmesh (`self.ItemMesh`))
  ;[0.8796 0.8228 0.05781 0.502] Highlight
  (bind _returnvalue (`GameplayStatics.GetActorOfClass` "/Game/Blueprints_Gameplay/BP_GameManager.BP_GameManager_C"))
  (if (== (`/Game/Blueprints_Gameplay/BP_GameManager.CurrentTaskGlow` _returnvalue) (`self.PasoRequerido`))
    (if (== (`self.IsGrabbed`) false)
      (`PrimitiveComponent.SetRenderCustomDepth` _itemmesh true)
      (else
        (`PrimitiveComponent.SetRenderCustomDepth` _itemmesh false :!label _label)))
    (else
      (goto _label))))

(event `self.GrabComponent.OnGrabbed`
  ;[0.5271 0.07227 0.07036 0.502] Foley
  (bind _returnvalue (`GameplayStatics.GetActorOfClass` "/Game/Audios/BP_AudioManagerMain.BP_AudioManagerMain_C"))
  (`/Game/Audios/BP_AudioManagerMain.PlayFoley` _returnvalue (`self.PropType`) (`self.K2_GetActorLocation`))
  (if (== (`/Game/Blueprints_Gameplay/BP_GameManager.CurrentTaskGlow` (stale `self.ReceiveTick` _returnvalue)) (`self.PasoRequerido`))
    (set `self.IsGrabbed` true)
    ;[0.8796 0.8228 0.05781 0.502] Highlight Central
    (`SceneComponent.SetVisibility` (`self.GetComponentByClass` (`self.TrigerDestino`) "/Script/Engine.StaticMeshComponent") true false)
    (`KismetSystemLibrary.Delay` 0.2)
    (`/Engine/EditorBlueprintResources/StandardMacros.DoOnce` false
      (:`Completed`
        ;[0.5271 0.07227 0.07036 0.502] Diálogo
        (bind _returnvalue_2 (`GameplayStatics.GetActorOfClass` "/Game/Audios/BP_AudioManagerMain.BP_AudioManagerMain_C"))
        (`/Game/Audios/BP_AudioManagerMain.PlayDialogue` _returnvalue_2 (`self.DialogueOnGrab`))))))

(event `self.GrabComponent.OnDropped`
  (set `self.IsGrabbed` false)
  (`SceneComponent.SetVisibility` (`self.GetComponentByClass` (`self.TrigerDestino`) "/Script/Engine.StaticMeshComponent") false false))

(fn `UserConstructionScript`)