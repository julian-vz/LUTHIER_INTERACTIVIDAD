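; Audio manager actor that centralizes the luthier's spoken dialogue and prop foley for a guitar-building experience.
; PlayDialogue maps a dialogue enum to main step instructions or extra lines, spawns the matching MetaSound at LuthierRef's root location and returns the audio component.
; PlayFoley maps a prop material enum (wood pitches, metal, glass, bulb) to a fire-and-forget sound at the given location.
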(event `self.ReceiveBeginPlay`)

(fn `PlayDialogue`
  (params (Type :type Byte))
  (returns (DialogueFinished :type "AudioComponent Object Reference"))
  (bind _returnvalue (`SceneComponent.K2_GetComponentLocation` (`/Game/Blueprints_Escenario/BP_ReferenciaLuthier.DefaultSceneRoot` (`self.Luthier_Ref`))))
  (switch `/Game/Audios/EN_DialogueTypeSound` (cast `/Game/Audios/EN_DialogueTypeSound` Type)
    (:`NewEnumerator17`
      (return null))
    (:`NewEnumerator0`
      ;[0.5271 0.07227 0.07036 0.502] Diálogos Principales
      (bind _returnvalue_2 (`GameplayStatics.SpawnSoundAtLocation` "/Game/Audios/Diálogos/MS_1InstrucciónTabla1.MS_1InstrucciónTabla1" _returnvalue (struct) 1.0 1.0 0.0 "/Game/Audios/SA_DiálogoLuthier.SA_DiálogoLuthier" null))
      (return _returnvalue_2))
    (:`NewEnumerator1`
      (bind _returnvalue_3 (`GameplayStatics.SpawnSoundAtLocation` "/Game/Audios/Diálogos/MS_2InstrucciónLija1.MS_2InstrucciónLija1" _returnvalue (struct) 1.0 1.0 0.0 "/Game/Audios/SA_DiálogoLuthier.SA_DiálogoLuthier" null))
      (return _returnvalue_3))
    (:`NewEnumerator2`
      (bind _returnvalue_4 (`GameplayStatics.SpawnSoundAtLocation` "/Game/Audios/Diálogos/MS_3InstrucciónVarillas1.MS_3InstrucciónVarillas1" _returnvalue (struct) 1.0 1.0 0.0 "/Game/Audios/SA_DiálogoLuthier.SA_DiálogoLuthier" null))
      (return _returnvalue_4))
    (:`NewEnumerator3`
      (bind _returnvalue_5 (`GameplayStatics.SpawnSoundAtLocation` "/Game/Audios/Diálogos/MS_4InstrucciónMástil1.MS_4InstrucciónMástil1" _returnvalue (struct) 1.0 1.0 0.0 "/Game/Audios/SA_DiálogoLuthier.SA_DiálogoLuthier" null))
      (return _returnvalue_5))
    (:`NewEnumerator4`
      (bind _returnvalue_6 (`GameplayStatics.SpawnSoundAtLocation` "/Game/Audios/Diálogos/MS_5InstrucciónAros1.MS_5InstrucciónAros1" _returnvalue (struct) 1.0 1.0 0.0 "/Game/Audios/SA_DiálogoLuthier.SA_DiálogoLuthier" null))
      (return _returnvalue_6))
    (:`NewEnumerator5`
      (bind _returnvalue_7 (`GameplayStatics.SpawnSoundAtLocation` "/Game/Audios/Diálogos/MS_6InstrucciónTrastes1.MS_6InstrucciónTrastes1" _returnvalue (struct) 1.0 1.0 0.0 "/Game/Audios/SA_DiálogoLuthier.SA_DiálogoLuthier" null))
      (return _returnvalue_7))
    (:`NewEnumerator6`
      (bind _returnvalue_8 (`GameplayStatics.SpawnSoundAtLocation` "/Game/Audios/Diálogos/MS_7InstrucciónBarniz1.MS_7InstrucciónBarniz1" _returnvalue (struct) 1.0 1.0 0.0 "/Game/Audios/SA_DiálogoLuthier.SA_DiálogoLuthier" null))
      (return _returnvalue_8))
    (:`NewEnumerator7`
      (bind _returnvalue_9 (`GameplayStatics.SpawnSoundAtLocation` "/Game/Audios/Diálogos/MS_8InstrucciónFinal.MS_8InstrucciónFinal" _returnvalue (struct) 1.0 1.0 0.0 "/Game/Audios/SA_DiálogoLuthier.SA_DiálogoLuthier" null))
      (return _returnvalue_9))
    (:`NewEnumerator11`
      ;[0.5271 0.07227 0.07036 0.502] Diálogos Extra
      (bind _returnvalue_10 (`GameplayStatics.SpawnSoundAtLocation` "/Game/Audios/Diálogos/MS_1InstrucciónTabla2.MS_1InstrucciónTabla2" _returnvalue (struct) 1.0 1.0 0.0 "/Game/Audios/SA_DiálogoLuthier.SA_DiálogoLuthier" null))
      (return _returnvalue_10))
    (:`NewEnumerator12`
      (bind _returnvalue_11 (`GameplayStatics.SpawnSoundAtLocation` "/Game/Audios/Diálogos/MS_2InstrucciónLija2.MS_2InstrucciónLija2" _returnvalue (struct) 1.0 1.0 0.0 "/Game/Audios/SA_DiálogoLuthier.SA_DiálogoLuthier" null))
      (return _returnvalue_11))
    (:`NewEnumerator13`
      (bind _returnvalue_12 (`GameplayStatics.SpawnSoundAtLocation` "/Game/Audios/Diálogos/MS_3InstrucciónVarillas2.MS_3InstrucciónVarillas2" _returnvalue (struct) 1.0 1.0 0.0 "/Game/Audios/SA_DiálogoLuthier.SA_DiálogoLuthier" null))
      (return _returnvalue_12))
    (:`NewEnumerator14`
      (bind _returnvalue_13 (`GameplayStatics.SpawnSoundAtLocation` "/Game/Audios/Diálogos/MS_4InstrucciónMástil2.MS_4InstrucciónMástil2" _returnvalue (struct) 1.0 1.0 0.0 "/Game/Audios/SA_DiálogoLuthier.SA_DiálogoLuthier" null))
      (return _returnvalue_13))
    (:`NewEnumerator15`
      (bind _returnvalue_14 (`GameplayStatics.SpawnSoundAtLocation` "/Game/Audios/Diálogos/MS_5InstrucciónAros2.MS_5InstrucciónAros2" _returnvalue (struct) 1.0 1.0 0.0 "/Game/Audios/SA_DiálogoLuthier.SA_DiálogoLuthier" null))
      (return _returnvalue_14))
    (:`NewEnumerator18`
      (bind _returnvalue_15 (`GameplayStatics.SpawnSoundAtLocation` "/Game/Audios/Diálogos/MS_6InstrucciónTrastes2.MS_6InstrucciónTrastes2" _returnvalue (struct) 1.0 1.0 0.0 "/Game/Audios/SA_DiálogoLuthier.SA_DiálogoLuthier" null))
      (return _returnvalue_15))
    (:`NewEnumerator16`
      (bind _returnvalue_16 (`GameplayStatics.SpawnSoundAtLocation` "/Game/Audios/Diálogos/MS_7InstrucciónBarniz2.MS_7InstrucciónBarniz2" _returnvalue (struct) 1.0 1.0 0.0 "/Game/Audios/SA_DiálogoLuthier.SA_DiálogoLuthier" null))
      (return _returnvalue_16))))

(fn `PlayFoley`
  (params (Type :type Byte) (Location :type "Vector Structure"))
  (switch `/Game/Audios/En_PropTypeSound` (cast `/Game/Audios/En_PropTypeSound` Type)
    (:`NewEnumerator0`
      (`GameplayStatics.PlaySoundAtLocation` "/Game/Audios/Foleys/MS_FoleyMaderaGrave.MS_FoleyMaderaGrave" Location (struct) 1.0 1.0 0.0 null null null null))
    (:`NewEnumerator1`
      (`GameplayStatics.PlaySoundAtLocation` "/Game/Audios/Foleys/MS_FoleyMaderaMedia.MS_FoleyMaderaMedia" Location (struct) 1.0 1.0 0.0 null null null null))
    (:`NewEnumerator2`
      (`GameplayStatics.PlaySoundAtLocation` "/Game/Audios/Foleys/MS_FoleyMaderaAguda.MS_FoleyMaderaAguda" Location (struct) 1.0 1.0 0.0 null null null null))
    (:`NewEnumerator3`
      (`GameplayStatics.PlaySoundAtLocation` "/Game/Audios/Foleys/MS_FoleyMetal.MS_FoleyMetal" Location (struct) 1.0 1.0 0.0 null null null null))
    (:`NewEnumerator4`
      (`GameplayStatics.PlaySoundAtLocation` "/Game/Audios/Foleys/MS_FoleyVidrio.MS_FoleyVidrio" Location (struct) 1.0 1.0 0.0 null null null null))
    (:`NewEnumerator5`
      (`GameplayStatics.PlaySoundAtLocation` "/Game/Audios/Foleys/MS_Foco.MS_Foco" Location (struct) 1.0 1.0 0.0 null null null null))))

(fn `UserConstructionScript`)