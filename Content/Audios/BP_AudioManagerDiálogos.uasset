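; Dialogue audio manager actor that plays voice lines for the steps of a luthier's instrument-building process, from soundboard to varnish and a final line.
; PlayDialogue switches on a dialogue type enum, spawns the matching main instruction or extra dialogue sound and returns its audio component.
; Only the first instruction plays at the LuthierRef actor's location; all others spawn at world origin.
; The event graph is empty.
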(fn `PlayDialogue`
  (params (Type :type Byte))
  (returns (DialogueFinished :type "AudioComponent Object Reference"))
  (switch `/Game/Audios/EN_DialogueTypeSound` (cast `/Game/Audios/EN_DialogueTypeSound` Type)
    (:`NewEnumerator17`
      (return null))
    (:`NewEnumerator0`
      ; Diálogos Principales
      (bind _returnvalue (`GameplayStatics.SpawnSoundAtLocation` "/Game/Audios/Diálogos/MS_1InstrucciónTabla1.MS_1InstrucciónTabla1" (`SceneComponent.K2_GetComponentLocation` (`/Game/Blueprints_Escenario/BP_ReferenciaLuthier.DefaultSceneRoot` (`self.Luthier_Ref`))) (struct) 1.0 1.0 0.0 "/Game/Audios/SA_DiálogoLuthier.SA_DiálogoLuthier" null))
      (return _returnvalue))
    (:`NewEnumerator1`
      (bind _returnvalue_2 (`GameplayStatics.SpawnSoundAtLocation` "/Game/Audios/Diálogos/MS_2InstrucciónLija1.MS_2InstrucciónLija1" (0.0 0.0 0.0) (struct) 1.0 1.0 0.0 "/Game/Audios/SA_DiálogoLuthier.SA_DiálogoLuthier" null))
      (return _returnvalue_2))
    (:`NewEnumerator2`
      (bind _returnvalue_3 (`GameplayStatics.SpawnSoundAtLocation` "/Game/Audios/Diálogos/MS_3InstrucciónVarillas1.MS_3InstrucciónVarillas1" (0.0 0.0 0.0) (struct) 1.0 1.0 0.0 "/Game/Audios/SA_DiálogoLuthier.SA_DiálogoLuthier" null))
      (return _returnvalue_3))
    (:`NewEnumerator3`
      (bind _returnvalue_4 (`GameplayStatics.SpawnSoundAtLocation` "/Game/Audios/Diálogos/MS_4InstrucciónMástil1.MS_4InstrucciónMástil1" (0.0 0.0 0.0) (struct) 1.0 1.0 0.0 "/Game/Audios/SA_DiálogoLuthier.SA_DiálogoLuthier" null))
      (return _returnvalue_4))
    (:`NewEnumerator4`
      (bind _returnvalue_5 (`GameplayStatics.SpawnSoundAtLocation` "/Game/Audios/Diálogos/MS_5InstrucciónAros1.MS_5InstrucciónAros1" (0.0 0.0 0.0) (struct) 1.0 1.0 0.0 "/Game/Audios/SA_DiálogoLuthier.SA_DiálogoLuthier" null))
      (return _returnvalue_5))
    (:`NewEnumerator5`
      (bind _returnvalue_6 (`GameplayStatics.SpawnSoundAtLocation` "/Game/Audios/Diálogos/MS_6InstrucciónTrastes1.MS_6InstrucciónTrastes1" (0.0 0.0 0.0) (struct) 1.0 1.0 0.0 "/Game/Audios/SA_DiálogoLuthier.SA_DiálogoLuthier" null))
      (return _returnvalue_6))
    (:`NewEnumerator6`
      (bind _returnvalue_7 (`GameplayStatics.SpawnSoundAtLocation` "/Game/Audios/Diálogos/MS_7InstrucciónBarniz1.MS_7InstrucciónBarniz1" (0.0 0.0 0.0) (struct) 1.0 1.0 0.0 "/Game/Audios/SA_DiálogoLuthier.SA_DiálogoLuthier" null))
      (return _returnvalue_7))
    (:`NewEnumerator7`
      (bind _returnvalue_8 (`GameplayStatics.SpawnSoundAtLocation` "/Game/Audios/Diálogos/MS_8InstrucciónFinal.MS_8InstrucciónFinal" (0.0 0.0 0.0) (struct) 1.0 1.0 0.0 "/Game/Audios/SA_DiálogoLuthier.SA_DiálogoLuthier" null))
      (return _returnvalue_8))
    (:`NewEnumerator11`
      ; Diálogos Extra
      (bind _returnvalue_9 (`GameplayStatics.SpawnSoundAtLocation` "/Game/Audios/Diálogos/MS_1InstrucciónTabla2.MS_1InstrucciónTabla2" (0.0 0.0 0.0) (struct) 1.0 1.0 0.0 "/Game/Audios/SA_DiálogoLuthier.SA_DiálogoLuthier" null))
      (return _returnvalue_9))
    (:`NewEnumerator12`
      (bind _returnvalue_10 (`GameplayStatics.SpawnSoundAtLocation` "/Game/Audios/Diálogos/MS_2InstrucciónLija2.MS_2InstrucciónLija2" (0.0 0.0 0.0) (struct) 1.0 1.0 0.0 "/Game/Audios/SA_DiálogoLuthier.SA_DiálogoLuthier" null))
      (return _returnvalue_10))
    (:`NewEnumerator13`
      (bind _returnvalue_11 (`GameplayStatics.SpawnSoundAtLocation` "/Game/Audios/Diálogos/MS_3InstrucciónVarillas2.MS_3InstrucciónVarillas2" (0.0 0.0 0.0) (struct) 1.0 1.0 0.0 "/Game/Audios/SA_DiálogoLuthier.SA_DiálogoLuthier" null))
      (return _returnvalue_11))
    (:`NewEnumerator14`
      (bind _returnvalue_12 (`GameplayStatics.SpawnSoundAtLocation` "/Game/Audios/Diálogos/MS_4InstrucciónMástil2.MS_4InstrucciónMástil2" (0.0 0.0 0.0) (struct) 1.0 1.0 0.0 "/Game/Audios/SA_DiálogoLuthier.SA_DiálogoLuthier" null))
      (return _returnvalue_12))
    (:`NewEnumerator15`
      (bind _returnvalue_13 (`GameplayStatics.SpawnSoundAtLocation` "/Game/Audios/Diálogos/MS_5InstrucciónAros2.MS_5InstrucciónAros2" (0.0 0.0 0.0) (struct) 1.0 1.0 0.0 "/Game/Audios/SA_DiálogoLuthier.SA_DiálogoLuthier" null))
      (return _returnvalue_13))
    (:`NewEnumerator16`
      (bind _returnvalue_14 (`GameplayStatics.SpawnSoundAtLocation` "/Game/Audios/Diálogos/MS_7InstrucciónBarniz2.MS_7InstrucciónBarniz2" (0.0 0.0 0.0) (struct) 1.0 1.0 0.0 "/Game/Audios/SA_DiálogoLuthier.SA_DiálogoLuthier" null))
      (return _returnvalue_14))))

(fn `UserConstructionScript`)